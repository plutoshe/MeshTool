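; BP_ToolMover relays the Ring character's tool events to its animation Blueprint, BP_RingAnimBP.
; On BeginPlay it casts the SuperMesh anim instance and caches it.
; Events for readying, disconnecting, using, finishing and switching tools write state flags and the incoming tool ID to that instance.
; Disconnect and finish reset their flag and the tool name, while the switching flag is only ever set here.
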(event `self.ReceiveBeginPlay`
  (bind _asbp_ring_anim_bp (cast `/Game/Characters/Ring/Animation/BP_RingAnimBP` (`SkeletalMeshComponent.GetAnimInstance` (`self.SuperMesh`))))
  (set `self.AnimationBP` _asbp_ring_anim_bp))

(event `self.BPGetToolReady`
  (params (toolID :type Name))
  (bind _animationbp (`self.AnimationBP`))
  (set `/Game/Characters/Ring/Animation/BP_RingAnimBP.m_Ready` true _animationbp)
  (set `/Game/Characters/Ring/Animation/BP_RingAnimBP.m_IncomeName` toolID _animationbp))

(event `self.BPDisconnectTool`
  (bind _animationbp (`self.AnimationBP`))
  (set `/Game/Characters/Ring/Animation/BP_RingAnimBP.m_Ready` false _animationbp)
  (set `/Game/Characters/Ring/Animation/BP_RingAnimBP.m_IncomeName` "None" _animationbp))

(event `self.BPUseTool`
  (params (toolID :type Name))
  (bind _animationbp (`self.AnimationBP`))
  (set `/Game/Characters/Ring/Animation/BP_RingAnimBP.m_Using` true _animationbp)
  (set `/Game/Characters/Ring/Animation/BP_RingAnimBP.m_IncomeName` toolID _animationbp))

(event `self.BPUseToolFinish`
  (bind _animationbp (`self.AnimationBP`))
  (set `/Game/Characters/Ring/Animation/BP_RingAnimBP.m_Using` false _animationbp)
  (set `/Game/Characters/Ring/Animation/BP_RingAnimBP.m_IncomeName` "None" _animationbp))

(event `self.BPSwitchTool`
  (params (toolID :type Name))
  (bind _animationbp (`self.AnimationBP`))
  (set `/Game/Characters/Ring/Animation/BP_RingAnimBP.m_SwitchingItem` true _animationbp)
  (set `/Game/Characters/Ring/Animation/BP_RingAnimBP.m_IncomeName` toolID _animationbp))

(fn `UserConstructionScript`)