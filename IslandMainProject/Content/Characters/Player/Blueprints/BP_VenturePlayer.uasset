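; BP_VenturePlayer is the player character Blueprint, which sets up the player's inventory window on BeginPlay.
; It creates an InventoryWindow widget from InventoryComp and its slot count, then adds it to the viewport.
; It then casts to BP_PlayerController and adds the widget to that controller's HUD canvas, auto-sized and anchored bottom-center.
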(event `self.ReceiveBeginPlay`
  (bind _inventorycomp (`self.InventoryComp`))
  ;[1 1 1] Inventory
  (`|ExecutionSequence`
    (:`then_0`
      (bind _returnvalue (`InventoryComponent.GetNumOfSlots` _inventorycomp))
      (bind _returnvalue_2 (`|CreateWidget` "/Game/UI/InventorySystem/InventoryUI/InventoryWindow.InventoryWindow_C" (`GameplayStatics.GetPlayerController` 0) _returnvalue _inventorycomp))
      (`UserWidget.AddToViewport` _returnvalue_2 0)
      (bind _asbp_player_controller (cast `/Game/Base/BP_PlayerController` (`GameplayStatics.GetPlayerController` 0)))
      (bind _returnvalue_3 (`CanvasPanel.AddChildToCanvas` (`/Game/UI/InventorySystem/InventoryUI/BP_HUD.HudCanvas` (`/Game/Base/BP_PlayerController.HUDWidget` _asbp_player_controller)) _returnvalue_2))
      (`CanvasPanelSlot.SetAutoSize` _returnvalue_3 true)
      (`CanvasPanelSlot.SetAlignment` _returnvalue_3 (0.5 0.0))
      (`CanvasPanelSlot.SetAnchors` _returnvalue_3 (make `Anchors` (0.5 0.9) (0.5 0.9))))))

(fn `UserConstructionScript`)