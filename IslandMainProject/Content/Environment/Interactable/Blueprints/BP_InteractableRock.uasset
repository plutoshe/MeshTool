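; BP_InteractableRock is an interactable environment rock that throws out its inventory items and kicks up dust when it drops.
; BPInteract calls ThrowAllItems on its Inventory.
; On actor overlap, a VenturePawn switches off physics simulation on OverlapComp.
; Otherwise, overlapping a StaticMeshActor spawns a dust emitter at a fixed offset below the rock, as a landing effect.
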(event `self.ReceiveActorBeginOverlap`
  (params (OtherActor :type "Actor Object Reference"))
  ;[1 1 1] Spawn smoke effect when it gets dropped down
  (cast `VenturePawn` OtherActor
    (:`then`
      (`PrimitiveComponent.SetSimulatePhysics` (`self.OverlapComp`) false))
    (:`CastFailed`
      (cast `StaticMeshActor` OtherActor)
      (`GameplayStatics.SpawnEmitterAtLocation` "/Game/ParticleSystem/P_DustEffect.P_DustEffect" (`KismetMathLibrary.MakeVector` (.x (`self.K2_GetActorLocation`)) (.y (`self.K2_GetActorLocation`)) (- (.z (`self.K2_GetActorLocation`)) 200.0))))))

(event `self.BPInteract`
  (`InventoryComponent.ThrowAllItems` (`self.Inventory`)))

(fn `UserConstructionScript`)