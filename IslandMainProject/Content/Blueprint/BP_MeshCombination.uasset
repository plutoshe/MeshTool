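; Actor that merges the static meshes of actors tagged "Mesh" into one combined mesh at BeginPlay.
; Each tagged actor of class aa has its mesh copied into the procedural mesh Addition, which serves as a scratch buffer for AddMesh with the world transform.
; The buffer is then cleared and the source actor destroyed.
; Pressing Y prints MMesh's section count and calls Smooth.
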(event `self.ReceiveBeginPlay`
  (`self.EnableInput` (`GameplayStatics.GetPlayerController` 0))
  (bind _outactors (`GameplayStatics.GetAllActorsWithTag` "Mesh"))
  (for _array_element _outactors
    (bind _asaa (cast `/Game/Blueprint/aa` _array_element))
    (bind _returnvalue (`self.GetComponentByClass` _asaa "/Script/Engine.StaticMeshComponent"))
    (`self.BPAddMesh` _returnvalue (`SceneComponent.K2_GetComponentToWorld` _returnvalue))
    (`self.K2_DestroyActor` _array_element)))

(event `self.ReceiveActorBeginOverlap`
  (params (OtherActor :type "Actor Object Reference")))

(event `Key|T`
  (params (Key :type "Key Structure")))

(event `Key|Y`
  (params (Key :type "Key Structure"))
  (:`Pressed`
    (`KismetSystemLibrary.PrintString` (`KismetStringLibrary.Conv_IntToString` (`ProceduralMeshComponent.GetNumSections` (`self.m_mesh`))))
    (`self.Smooth`)))

(fn `BPAddMesh`
  (params (StaticMeshComp :type "StaticMeshComponent Object Reference") (LocalTransrform :type "Transform Structure"))
  (bind _addition (`self.Addition`))
  (`KismetProceduralMeshLibrary.CopyProceduralMeshFromStaticMeshComponent` StaticMeshComp 0 _addition)
  (if (`KismetSystemLibrary.IsValid` _addition)
    (`KismetSystemLibrary.PrintString` (`KismetStringLibrary.Conv_IntToString` (`ProceduralMeshComponent.GetNumSections` _addition)))
    (`self.AddMesh` _addition LocalTransrform)
    (`ProceduralMeshComponent.ClearAllMeshSections` _addition)
    (return)))

(fn `UserConstructionScript`)