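; Test actor that turns its static mesh component into a procedural mesh at BeginPlay and adds a flat quad to it.
; It copies the static mesh with collision, appends the hardcoded quad as a new section, then destroys the static mesh component.
; For debugging, it reads back section index 3 and prints its triangle index count and first vertex.
; The construction script does nothing, as its quad-creation node is unconnected.
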(event `self.ReceiveBeginPlay`
  (bind _staticmesh (`self.StaticMesh`))
  (bind _proceduralmesh (`self.ProceduralMesh`))
  (`KismetProceduralMeshLibrary.CopyProceduralMeshFromStaticMeshComponent` _staticmesh 0 _proceduralmesh true)
  (`ProceduralMeshComponent.CreateMeshSection_LinearColor` :`self` _proceduralmesh :`SectionIndex` (`ProceduralMeshComponent.GetNumSections` _proceduralmesh) :`Vertices` (`|MakeArray` (0.0 0.0 0.0) (0.0 100.0 0.0) (100.0 0.0 0.0) (100.0 100.0 0.0) :!type "Vector Structure") :`Triangles` (`|MakeArray` 0 1 2 3 2 1) :`UV0` (`|MakeArray` (0.0 0.0) (0.0 1.0) (1.0 0.0) (1.0 1.0) :!type "Vector2D Structure"))
  (`ActorComponent.K2_DestroyComponent` _staticmesh)
  (bind (_vertices _triangles) (`KismetProceduralMeshLibrary.GetSectionFromProceduralMesh` _proceduralmesh 3))
  (`KismetSystemLibrary.PrintString` (`KismetStringLibrary.Conv_IntToString` (`KismetArrayLibrary.Array_Length` _triangles)))
  (`KismetSystemLibrary.PrintString` (`KismetStringLibrary.Conv_VectorToString` (`|GetArrayItem` _vertices))))

(fn `UserConstructionScript`)