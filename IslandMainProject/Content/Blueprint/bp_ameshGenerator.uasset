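; Mesh generator actor that, on pressing T, absorbs "Mesh"-tagged actors of class aa and destroys them.
; Each one's StaticMeshComponent goes to BPAddMesh with its world location offset from the generator, carrying no rotation or scale.
; BPAddMesh copies it into ProceduralMesh1 as a scratch buffer, passes that to AddMesh, then clears it for reuse.
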(event `self.ReceiveBeginPlay`
  (`self.EnableInput` (`GameplayStatics.GetPlayerController` 0)))

(event `self.ReceiveActorBeginOverlap`
  (params (OtherActor :type "Actor Object Reference")))

(event `Key|T`
  (params (Key :type "Key Structure"))
  (:`Pressed`
    (bind _outactors (`GameplayStatics.GetAllActorsWithTag` "Mesh"))
    (for _array_element _outactors
      (bind _asaa (cast `/Game/Blueprint/aa` _array_element))
      (bind _returnvalue (`self.GetComponentByClass` _asaa "/Script/Engine.StaticMeshComponent"))
      (`self.BPAddMesh` _returnvalue (`KismetMathLibrary.Conv_VectorToTransform` (- (`SceneComponent.K2_GetComponentLocation` _returnvalue) (`self.K2_GetActorLocation`))))
      (`self.K2_DestroyActor` _array_element))))

(fn `BPAddMesh`
  (params (StaticMesh :type "StaticMeshComponent Object Reference") (LocalTransform :type "Transform Structure"))
  (bind _proceduralmesh1 (`self.ProceduralMesh1`))
  (`KismetProceduralMeshLibrary.CopyProceduralMeshFromStaticMeshComponent` StaticMesh 0 _proceduralmesh1)
  (if (`KismetSystemLibrary.IsValid` _proceduralmesh1)
    (`self.AddMesh` _proceduralmesh1 LocalTransform)
    (`ProceduralMeshComponent.ClearAllMeshSections` _proceduralmesh1)
    (return)))

(fn `UserConstructionScript`)